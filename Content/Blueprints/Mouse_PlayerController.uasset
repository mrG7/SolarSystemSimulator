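; Player controller for mouse input that lets the player look around and select planets by clicking.
; Holding left mouse hides the cursor and enables yaw and pitch rotation from the Turn and LookUp axes.
; A press traces under the cursor and stores any Planet-tagged actor as the Observer pawn's selection.
; Release restores the cursor and notifies every HUD_Interface and BasePlanet actor; construction sets a downward-angled starting rotation.
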(event `Key|LeftMouseButton` :paused true
  (params (Key :type "Key Structure" :default "AnyKey"))
  (bind (_hitresult _returnvalue) (`self.GetHitResultUnderCursorByChannel` "TraceTypeQuery1"))
  (bind (_bblockinghit _binitialoverlap _time _location _impactpoint _normal _impactnormal _physmat _hitactor) (`GameplayStatics.BreakHitResult` _hitresult))
  ;[1 1 1] Left Mouse Conditions
  (:`Pressed`
    (set `self.Mouse Press` true)
    (set `self.bShowMouseCursor` false)
    ;[1 1 1] Move Player to the Planet when click them
    (if _returnvalue
      (if (`self.ActorHasTag` _hitactor "Planet")
        (bind _asobserver (cast `/Game/Blueprints/Observer` (`self.K2_GetPawn`)))
        (set `/Game/Blueprints/Observer.ActorSelected` _hitactor _asobserver))))
  (:`Released`
    (`|ExecutionSequence`
      (:`then_0`
        (set `self.Mouse Press` false)
        (set `self.bShowMouseCursor` true))
      (:`then_1`
        (bind _outactors (`GameplayStatics.GetAllActorsOfClass` "/Game/Blueprints/HUD_Interface.HUD_Interface_C"))
        (for _array_element _outactors
          (bind _ashud_interface (cast `/Game/Blueprints/HUD_Interface` _array_element))
          (`/Game/Blueprints/HUD_Interface.MouseClickRelease` _ashud_interface)))
      (:`then_2`
        (bind _outactors_2 (`GameplayStatics.GetAllActorsOfClass` "/Game/Blueprints/BasePlanet.BasePlanet_C"))
        (for _array_element_2 _outactors_2
          (bind _asbase_planet (cast `/Game/Blueprints/BasePlanet` _array_element_2))
          (`/Game/Blueprints/BasePlanet.Mouse Release Event` _asbase_planet))))))

(event `InputAxis|Turn` :overrideparent false
  (params (AxisValue :type "Float (single-precision)"))
  ;[1 1 1] Camera Rotation Controls
  (if (`self.Mouse Press`)
    (`self.AddYawInput` AxisValue)))

(event `InputAxis|LookUp` :overrideparent false
  (params (AxisValue :type "Float (single-precision)"))
  ;[1 1 1] Camera Rotation Controls
  (if (`self.Mouse Press`)
    (`self.AddPitchInput` AxisValue)))

(fn `UserConstructionScript`
  (`self.SetControlRotation` (`KismetMathLibrary.MakeRotator` 0.0 -45.0 0.0)))