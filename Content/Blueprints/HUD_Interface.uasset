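; HUD for a solar system simulation, drawing a control bar, quit button and custom mouse cursor.
; DrawHUD scales textures and named hit boxes from a 1920x1080 layout, choosing textures by hover and toggle state.
; Clicks set play/pause state, quit, or call visibility, sound and reset events on all matching sun, planet, orbit and gravity field actors.
; A draggable scroller follows the mouse and drives a looked-up audio pitch every Tick.
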(event `self.ReceiveHitBoxBeginCursorOver`
  (params (BoxName :type Name))
  ;[1 1 1] Commands and Sounds
  ;;[1 1 1] Buttons Highlights andothers
  (`self.Highlight Button On` BoxName)
  ;;[1 1 1] Menu Hover Sound
  (`GameplayStatics.PlaySoundAtLocation` "/Game/Audio/Menu_Hover.Menu_Hover" (`Pawn.GetNavAgentLocation` (`GameplayStatics.GetPlayerPawn` 0))))

(event `self.ReceiveHitBoxEndCursorOver`
  (params (BoxName :type Name))
  ;[1 1 1] Commands and Sounds
  ;;[1 1 1] Buttons Highlights andothers
  (`self.Highlight Button Off` BoxName))

(event `self.ReceiveHitBoxRelease`
  (params (BoxName :type Name))
  ;[1 1 1] Commands and Sounds
  ;;[1 1 1] Buttons Highlights andothers
  (`self.Highlight Button On` BoxName :!label _label)
  (`AudioComponent.Stop` (`self.Audio1`)))

(event `MouseClickRelease`
  ;[1 1 1] Commands and Sounds
  ;;[1 1 1] Buttons Highlights andothers
  (set `self.ScroolerClick` false)
  (goto _label))

(event `self.ReceiveHitBoxClick`
  (params (BoxName :type Name))
  ;[1 1 1] Commands and Sounds
  (`|ExecutionSequence`
    (:`then_0`
      ;;[1 1 1] Menu Click Sound
      (`GameplayStatics.PlaySoundAtLocation` "/Game/Audio/Menu_Click.Menu_Click" (`Pawn.GetNavAgentLocation` (`GameplayStatics.GetPlayerPawn` 0))))
    (:`then_1`
      (switch `name` BoxName
        (:`Play`
          ;;[1 1 1] Play
          (set `self.Play_B_Clicked` false))
        (:`Pause`
          ;;[1 1 1] Pause
          (set `self.Play_B_Clicked` true))
        (:`Text`
          ;;[1 1 1] Planets Vis
          (`|ExecutionSequence`
            (:`then_0`
              (bind _outactors (`GameplayStatics.GetAllActorsOfClass` "/Game/Actors_Blueprints/SunBlueprint.SunBlueprint_C"))
              (for _array_element _outactors
                (bind _assunblueprint_c (cast `/Game/Actors_Blueprints/SunBlueprint` _array_element))
                (`/Game/Actors_Blueprints/SunBlueprint.TextVisibilityEvent` _assunblueprint_c)))
            (:`then_1`
              (bind _outactors_2 (`GameplayStatics.GetAllActorsOfClass` "/Game/Blueprints/BasePlanet.BasePlanet_C"))
              (for _array_element_2 _outactors_2
                (bind _asbaseplanet_c (cast `/Game/Blueprints/BasePlanet` _array_element_2))
                (`/Game/Blueprints/BasePlanet.TextVisTrigger` _asbaseplanet_c))
              (bind _isa (`/Engine/EditorBlueprintResources/StandardMacros.FlipFlop`)
                (:`A`
                  _)
                (:`B`
                  _))
              (set `self.TextVis_B_Clicked` _isa))))
        (:`Orbit`
          ;;[1 1 1] Orbit
          (bind _outactors_3 (`GameplayStatics.GetAllActorsOfClass` "/Game/Actors_Blueprints/Orbits.Orbits_C" :!label _label_2))
          (for _array_element_3 _outactors_3
            (bind _asorbits_c (cast `/Game/Actors_Blueprints/Orbits` _array_element_3))
            (`/Game/Actors_Blueprints/Orbits.OrbitVisibility` _asorbits_c))
          (bind _isa_2 (`/Engine/EditorBlueprintResources/StandardMacros.FlipFlop`)
            (:`A`
              _)
            (:`B`
              _))
          (set `self.OrbitVis_B_Clicked` _isa_2))
        (:`Gravity`
          ;;[1 1 1] Gravity Field
          (bind _outactors_4 (`GameplayStatics.GetAllActorsOfClass` "/Game/Actors_Blueprints/GravityField.GravityField_C"))
          (for _array_element_4 _outactors_4
            (bind _asgravityfield_c (cast `/Game/Actors_Blueprints/GravityField` _array_element_4))
            (`/Game/Actors_Blueprints/GravityField.GravityVisibility` _asgravityfield_c))
          (bind _isa_3 (`/Engine/EditorBlueprintResources/StandardMacros.FlipFlop`)
            (:`A`
              _)
            (:`B`
              _))
          (set `self.Gravity_B_Cliked` _isa_3))
        (:`Reset`
          ;;[1 1 1] Reset
          (`|ExecutionSequence` :!label _label_3
            (:`then_0`
              (bind _outactors_5 (`GameplayStatics.GetAllActorsOfClass` "/Game/Blueprints/BasePlanet.BasePlanet_C"))
              (for _array_element_5 _outactors_5
                (bind _asbaseplanet_c_2 (cast `/Game/Blueprints/BasePlanet` _array_element_5))
                (`/Game/Blueprints/BasePlanet.ResetTrigger` _asbaseplanet_c_2)))
            (:`then_1`
              (goto _label_4 :!via `Reset`))))
        (:`Scroller`
          ;;[1 1 1] Scroller
          (set `self.ScroolerClick` true)
          (`AudioComponent.Play` (`self.Audio1`) 0.0))
        (:`Sound`
          ;;[1 1 1] Planets Sound Trigger
          (bind _outactors_6 (`GameplayStatics.GetAllActorsOfClass` "/Game/Blueprints/BasePlanet.BasePlanet_C"))
          (for _array_element_6 _outactors_6
            (bind _asbaseplanet_c_3 (cast `/Game/Blueprints/BasePlanet` _array_element_6))
            (`/Game/Blueprints/BasePlanet.SoundTrigger` _asbaseplanet_c_3))
          (bind _isa_4 (`/Engine/EditorBlueprintResources/StandardMacros.FlipFlop`)
            (:`A`
              _)
            (:`B`
              _))
          (set `self.Sound Vis B Clicked` _isa_4))
        (:`Quit`
          (`KismetSystemLibrary.QuitGame` null))))))

(event `self.ReceiveDrawHUD`
  (params (SizeX :type Integer) (SizeY :type Integer))
  (bind _returnvalue (`GameplayStatics.GetPlayerController` 0))
  (bind _play_b_clicked (`self.Play_B_Clicked`))
  (bind _play_b_clicked_2 (`self.Play_B_Clicked`))
  (bind _sound_vis_b_clicked (`self.Sound Vis B Clicked`))
  (bind _gravity_b_cliked (`self.Gravity_B_Cliked`))
  (bind _orbitvis_b_clicked (`self.OrbitVis_B_Clicked`))
  (bind (_locationx _locationy) (`PlayerController.GetMousePosition` _returnvalue))
  (bind (_sizex _sizey) (`PlayerController.GetViewportSize` _returnvalue))
  (bind _returnvalue_2 (/ 50.0 2.0))
  (bind _returnvalue_3 (`KismetMathLibrary.FInterpEaseInOut` (`KismetMathLibrary.BreakVector2D` (`self.ScrollerLocation`)) (`KismetMathLibrary.FClamp` (- (`PlayerController.GetMousePosition` (`GameplayStatics.GetPlayerController` 0)) 18.0) (`KismetMathLibrary.BreakVector2D` (`self.ScrollerStart`)) (* (`KismetMathLibrary.Conv_IntToDouble` (`PlayerController.GetViewportSize` (`GameplayStatics.GetPlayerController` 0))) 0.7992)) (select `bool` (`self.ScroolerClick`) :`true` 1.0 :!type "Float (single-precision)") 1.0))
  (bind _returnvalue_4 (`KismetMathLibrary.MakeVector2D` _returnvalue_3))
  ;[1 1 1] Drawning
  (set `self.Screen Dimension` (`KismetMathLibrary.MakeVector2D` (`KismetMathLibrary.Conv_IntToDouble` SizeX) (`KismetMathLibrary.Conv_IntToDouble` SizeY)))
  (`|ExecutionSequence`
    (:`then_0`
      ;;[1 1 1] Play / Pause
      (bind (_outpux _outputy _outscale) (`self.Scaleto Ratio` 394.0 940.0 0.39))
      (`self.DrawButton` _outpux _outputy "Play" (select `bool` (`self.PlayHover`) :`false` (select `bool` _play_b_clicked_2 :`false` "/Game/Textures/HUD/B_Play6on.B_Play6on" :`true` "/Game/Textures/HUD/B_Play6.B_Play6" :!type "Texture2D Object Reference") :`true` (select `bool` _play_b_clicked_2 :`false` "/Game/Textures/HUD/B_Play6hon.B_Play6hon" :`true` "/Game/Textures/HUD/B_Play6h.B_Play6h" :!type "Texture2D Object Reference")) "" _outscale (* (128.0 128.0) _outscale)))
    (:`then_1`
      (bind (_outpux_2 _outputy_2 _outscale_2) (`self.Scaleto Ratio` 440.0 940.0 0.39))
      (`self.DrawButton` _outpux_2 _outputy_2 "Pause" (select `bool` (`self.PauseHover`) :`false` (select `bool` _play_b_clicked :`false` "/Game/Textures/HUD/B_Pause.B_Pause" :`true` "/Game/Textures/HUD/B_Pauseon.B_Pauseon" :!type "Texture2D Object Reference") :`true` (select `bool` _play_b_clicked :`false` "/Game/Textures/HUD/B_Pauseh.B_Pauseh" :`true` "/Game/Textures/HUD/B_Pausehon.B_Pausehon" :!type "Texture2D Object Reference")) "" _outscale_2 (* (128.0 128.0) _outscale_2)))
    (:`then_2`
      ;;[1 1 1] Reset
      (bind (_outpux_3 _outputy_3 _outscale_3) (`self.Scaleto Ratio` 488.0 940.0 0.68))
      (`self.DrawButton` _outpux_3 _outputy_3 "Reset" (select `bool` (`self.ResetHover`) :`false` "/Game/Textures/HUD/B_Reset2.B_Reset2" :`true` "/Game/Textures/HUD/B_ResetH2.B_ResetH2" :!type "Texture2D Object Reference") "" _outscale_3 (* (128.0 76.0) _outscale_3)))
    (:`then_3`
      ;;[1 1 1] Slider + Scroller
      (bind (_outpux_4 _outputy_4 _outscale_4) (`self.Scaleto Ratio` 300.0 990.0 1.0))
      (`self.DrawButton` _outpux_4 _outputy_4 "Slider" "/Game/Textures/HUD/Slider_2.Slider_2" "" _outscale_4 (0.0 0.0)))
    (:`then_4`
      ;;[1 1 1] Mouse Cursor
      (bind _asmouse_playercontroller_c (cast `/Game/Blueprints/Mouse_PlayerController` (`GameplayStatics.GetPlayerController` 0)))
      (if (not (`/Game/Blueprints/Mouse_PlayerController.Mouse Press` _asmouse_playercontroller_c))
        (`self.DrawMaterial` "/Game/Textures/HUD/Mouse_Cursor_Mat.Mouse_Cursor_Mat" (- (+ (/ (`KismetMathLibrary.Conv_IntToDouble` (- SizeX _sizex)) 2.0) _locationx) _returnvalue_2) (- (+ (/ (`KismetMathLibrary.Conv_IntToDouble` (- SizeY _sizey)) 2.0) _locationy) _returnvalue_2) 50.0 50.0 0.0 0.0 1.0 1.0)))
    (:`then_5`
      ;;[1 1 1] Visibility
      (bind (_outpux_5 _outputy_5 _outscale_5) (`self.Scaleto Ratio` 573.0 943.0 0.52))
      (`self.DrawButton` _outpux_5 _outputy_5 "Text" (select `bool` (`self.TextVis_Hover`) :`false` (select `bool` (`self.TextVis_B_Clicked`) :`false` "/Game/Textures/HUD/B_Text_On4.B_Text_On4" :`true` "/Game/Textures/HUD/B_Text_On4off.B_Text_On4off" :!type "Texture2D Object Reference") :`true` (select `bool` (`self.TextVis_B_Clicked`) :`false` "/Game/Textures/HUD/B_Text_On4_H.B_Text_On4_H" :`true` "/Game/Textures/HUD/B_Text_On4off_H.B_Text_On4off_H" :!type "Texture2D Object Reference")) "" _outscale_5 (* (120.0 78.0) _outscale_5)))
    (:`then_6`
      (bind (_outpux_6 _outputy_6 _outscale_6) (`self.Scaleto Ratio` 643.0 943.0 0.52))
      (`self.DrawButton` _outpux_6 _outputy_6 "Orbit" (select `bool` (`self.oRBITvIS`) :`false` (select `bool` _orbitvis_b_clicked :`false` "/Game/Textures/HUD/B_OrbitOn.B_OrbitOn" :`true` "/Game/Textures/HUD/B_OrbitOff.B_OrbitOff" :!type "Texture2D Object Reference") :`true` (select `bool` _orbitvis_b_clicked :`false` "/Game/Textures/HUD/B_OrbitOn_H.B_OrbitOn_H" :`true` "/Game/Textures/HUD/B_OrbitOff_H.B_OrbitOff_H" :!type "Texture2D Object Reference")) "" _outscale_6 (* (120.0 78.0) _outscale_6)))
    (:`then_7`
      (bind (_outpux_7 _outputy_7 _outscale_7) (`self.Scaleto Ratio` 712.0 943.0 0.52))
      (`self.DrawButton` _outpux_7 _outputy_7 "Gravity" (select `bool` (`self.GravityVis`) :`false` (select `bool` _gravity_b_cliked :`false` "/Game/Textures/HUD/B_GravityOn.B_GravityOn" :`true` "/Game/Textures/HUD/B_GravityOff.B_GravityOff" :!type "Texture2D Object Reference") :`true` (select `bool` _gravity_b_cliked :`false` "/Game/Textures/HUD/B_GravityOn_H.B_GravityOn_H" :`true` "/Game/Textures/HUD/B_GravityOff_H.B_GravityOff_H" :!type "Texture2D Object Reference")) "" _outscale_7 (* (120.0 78.0) _outscale_7)))
    (:`then_8`
      ;;[1 1 1] Quit
      (bind (_outpux_8 _outputy_8 _outscale_8) (`self.Scaleto Ratio` 1760.0 50.0 0.1))
      (`self.DrawButton` _outpux_8 _outputy_8 "Quit" (select `bool` (`self.QuitHover`) :`false` "/Game/Textures/HUD/QuitButton.QuitButton" :`true` "/Game/Textures/HUD/QuitButton_H.QuitButton_H" :!type "Texture2D Object Reference") "" _outscale_8 (* (1024.0 512.0) _outscale_8)))
    (:`then_9`
      (bind (_outpux_9 _outputy_9 _outscale_9) (`self.Scaleto Ratio` 938.0 1005.0 1.0))
      (`|ExecutionSequence`
        (:`then_0`
          (bind _returnvalue_5 (`KismetMathLibrary.MakeVector2D` _outpux_9 _outputy_9))
          (`self.ScrollerOutputvalue` _returnvalue_5)
          (`self.DrawButton` _returnvalue_3 _outputy_9 "Scroller" (select `bool` (`self.ScrollerHover`) :`false` "/Game/Textures/HUD/Scroller.Scroller" :`true` "/Game/Textures/HUD/ScrollerH2.ScrollerH2" :!type "Texture2D Object Reference") "" _outscale_9 (* (45.0 45.0) _outscale_9))
          (set `self.ScrollerValuesExp` (`KismetMathLibrary.BreakVector2D` _returnvalue_4))
          (if (`self.ScroolerClick`)
            (set `self.ScrollerLocation` _returnvalue_4)))
        (:`then_1`
          (`/Engine/EditorBlueprintResources/StandardMacros.DoOnce` false :!label _label_4
            (:`Completed`
              (set `self.ScrollerLocation` _returnvalue_5)
              (set `self.ScrollerStartLocation` _returnvalue_5))))))
    (:`then_10`
      (bind (_outpux_10 _outputy_10 _outscale_10) (`self.Scaleto Ratio` 781.0 943.0 0.52))
      (`self.DrawButton` _outpux_10 _outputy_10 "Sound" (select `bool` (`self.Sound Vis B Hover`) :`false` (select `bool` _sound_vis_b_clicked :`false` "/Game/Textures/HUD/B_SoundOn.B_SoundOn" :`true` "/Game/Textures/HUD/B_SoundOff.B_SoundOff" :!type "Texture2D Object Reference") :`true` (select `bool` _sound_vis_b_clicked :`false` "/Game/Textures/HUD/B_SoundOn_H.B_SoundOn_H" :`true` "/Game/Textures/HUD/B_SoundOff_H.B_SoundOff_H" :!type "Texture2D Object Reference")) "" _outscale_10 (* (120.0 78.0) _outscale_10)))))

(event `Trigger from Panels`
  ;[1 1 1] Commands and Sounds
  ;;[1 1 1] Orbit
  (goto _label_2))

(event `self.ReceiveBeginPlay`
  ;[1 1 1] Commands and Sounds
  (`|ExecutionSequence`
    (:`then_0`
      (`KismetSystemLibrary.Delay` 1.0)
      (goto _label_3))
    (:`then_1`
      ;;[1 1 1] Scroller
      (`AudioComponent.SetSound` (`self.Audio1`) "/Game/Audio/Click03_Cue.Click03_Cue"))))

(event `self.ReceiveTick`
  (params (DeltaSeconds :type "Float (single-precision)"))
  ;[1 1 1] Drawning
  ;;[1 1 1] Slider + Scroller
  (`AudioComponent.SetPitchMultiplier` (`self.Audio1`) (`KismetMathLibrary.Abs` (/ (- (`KismetMathLibrary.BreakVector2D` (`KismetMathLibrary.MakeVector2D` (`KismetMathLibrary.FInterpEaseInOut` (`KismetMathLibrary.BreakVector2D` (`self.ScrollerLocation`)) (`KismetMathLibrary.FClamp` (- (`PlayerController.GetMousePosition` (`GameplayStatics.GetPlayerController` 0)) 18.0) (`KismetMathLibrary.BreakVector2D` (`self.ScrollerStart`)) (* (`KismetMathLibrary.Conv_IntToDouble` (`PlayerController.GetViewportSize` (`GameplayStatics.GetPlayerController` 0))) 0.7992)) (select `bool` (`self.ScroolerClick`) :`true` 1.0 :!type "Float (single-precision)") 1.0))) 630.0) 400.0))))

(fn `ClickCaller`
  (params (`Actor Class` :type "Actor Class Reference") (`Hit Box Name` :type Name))
  (returns (`Array Eelement` :type "Object Object Reference"))
  (switch `name` `Hit Box Name`
    (:`Text`
      (bind _outactors (`GameplayStatics.GetAllActorsOfClass` `Actor Class`))
      (for _array_element _outactors
        (return _array_element)))))

(fn `DrawButton`
  (params (`Location X` :type "Float (double-precision)") (`Location  Y` :type "Float (double-precision)") (`HitBox Name` :type Name) (ButtonTexture :type "Texture2D Object Reference") (Text :type String) (Scale :type "Float (double-precision)") (`Size of Hitbox` :type "Object.Vector2D Structure"))
  (`self.DrawTextureSimple` ButtonTexture `Location X` `Location  Y` Scale)
  (`self.AddHitBox` (`KismetMathLibrary.MakeVector2D` `Location X` `Location  Y`) `Size of Hitbox` `HitBox Name`))

(fn `DrawButtonFix`
  (params (`Location X` :type "Float (double-precision)") (`Location  Y` :type "Float (double-precision)") (`HitBox Name` :type Name) (ButtonTexture :type "Texture2D Object Reference") (Scale :type "Float (double-precision)"))
  (`self.DrawTexture` ButtonTexture `Location X` `Location  Y` 0.0 0.0 0.0 0.0 0.0 0.0 (struct :`R` 1.0 :`G` 1.0 :`B` 1.0 :`A` 1.0) "BLEND_Translucent" Scale)
  (`self.AddHitBox` (`KismetMathLibrary.MakeVector2D` `Location X` `Location  Y`) (/ (0.0 0.0) Scale) `HitBox Name`))

(fn `DrawMaterialButtom`
  (params (Material :type "Material Object Reference") (`Screen X` :type "Float (double-precision)") (`Screen Y` :type "Float (double-precision)") (`Screen W` :type "Float (double-precision)") (`Screen H` :type "Float (double-precision)") (Scale :type "Float (double-precision)"))
  (returns (Position :type "Object.Vector2D Structure") (Size :type "Object.Vector2D Structure"))
  (`self.DrawMaterialSimple` Material `Screen X` `Screen Y` `Screen W` `Screen H` Scale)
  (return (`KismetMathLibrary.MakeVector2D` `Screen X` `Screen Y`) (`KismetMathLibrary.MakeVector2D` `Screen W` `Screen H`)))

(fn `Highlight Button Clicked`
  (params (`Hit Box name` :type Name))
  (switch `name` `Hit Box name`
    (:`Play`
      (set `self.PlayClick` true))))

(fn `Highlight Button Not Clicked`
  (params (`Hit Box name` :type Name))
  (switch `name` `Hit Box name`
    (:`Play`
      (set `self.PlayClick` false))))

(fn `Highlight Button Off`
  (params (`Hit Box name` :type Name))
  (switch `name` `Hit Box name`
    (:`Play`
      (set `self.PlayHover` false))
    (:`Pause`
      (set `self.PauseHover` false))
    (:`Text`
      (set `self.TextVis_Hover` false))
    (:`Orbit`
      (set `self.oRBITvIS` false))
    (:`Gravity`
      (set `self.GravityVis` false))
    (:`Reset`
      (set `self.ResetHover` false))
    (:`Scroller`
      (set `self.ScrollerHover` false))
    (:`Sound`
      (set `self.Sound Vis B Hover` false))
    (:`Quit`
      (set `self.QuitHover` false))))

(fn `Highlight Button On`
  (params (`Hit Box name` :type Name))
  (switch `name` `Hit Box name`
    (:`Play`
      (set `self.PlayHover` true))
    (:`Pause`
      (set `self.PauseHover` true))
    (:`Text`
      (set `self.TextVis_Hover` true))
    (:`Orbit`
      (set `self.oRBITvIS` true))
    (:`Gravity`
      (set `self.GravityVis` true))
    (:`Reset`
      (set `self.ResetHover` true))
    (:`Scroller`
      (set `self.ScrollerHover` true))
    (:`Sound`
      (set `self.Sound Vis B Hover` true))
    (:`Quit`
      (set `self.QuitHover` true))))

(fn `NewFunction`)

(fn `Scaleto Ratio`
  (params (InputX :type "Float (double-precision)") (InputY :type "Float (double-precision)") (InScale :type "Float (double-precision)"))
  (returns (OutpuX :type "Float (double-precision)") (OutputY :type "Float (double-precision)") (OutScale :type "Float (double-precision)"))
  (bind _ratioy (`self.RatioY`))
  (bind (_sizex _sizey) (`PlayerController.GetViewportSize` (`GameplayStatics.GetPlayerController` 0)))
  (bind (_x _y) (`KismetMathLibrary.BreakVector2D` (`self.Screen Dimension`)))
  (set `self.Screen Dimension` (`KismetMathLibrary.MakeVector2D` (`KismetMathLibrary.Conv_IntToDouble` _sizex) (`KismetMathLibrary.Conv_IntToDouble` _sizey)))
  (`|ExecutionSequence`
    (:`then_0`
      (set `self.RatioX` (/ _x 1920.0)))
    (:`then_1`
      (set `self.RatioY` (/ _y 1080.0)))
    (:`then_2`
      (return (* InputX (`self.RatioX`)) (* InputY _ratioy) (* InScale _ratioy)))))

(fn `ScrollerOutputvalue`
  (params (`Relative Location` :type "Object.Vector2D Structure"))
  (set `self.Value` (/ (`KismetMathLibrary.VSize2D` (- `Relative Location` (`self.ScrollerStart`))) (`KismetMathLibrary.VSize2D` (- (`self.ScrollerEnd`) (`self.ScrollerStart`))))))

(fn `UserConstructionScript`)