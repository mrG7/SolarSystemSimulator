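; BasePlanet is a planet actor Blueprint, named as a base class, that handles clicks and holds toggle state.
; Clicking it plays the PlanetClick sound at the player pawn's nav agent location.
; Three trigger events use FlipFlops to toggle the SoundButton, ResetRigger and TextVisibility variables, with nothing wired to either branch.
; MouseReleaseEvent, InfoPanel and the construction script are empty.
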(event `Mouse Release Event`)

(event `self.ReceiveActorOnClicked`
  (`GameplayStatics.PlaySoundAtLocation` "/Game/Audio/PlanetClick.PlanetClick" (`Pawn.GetNavAgentLocation` (`GameplayStatics.GetPlayerPawn` 0))))

(event `SoundTrigger`
  (bind _isa (`/Engine/EditorBlueprintResources/StandardMacros.FlipFlop`)
    (:`A`
      _)
    (:`B`
      _))
  (set `self.SoundButton` _isa))

(event `ResetTrigger`
  (bind _isa (`/Engine/EditorBlueprintResources/StandardMacros.FlipFlop`)
    (:`A`
      _)
    (:`B`
      _))
  (set `self.ResetRigger` _isa))

(event `TextVisTrigger`
  (bind _isa (`/Engine/EditorBlueprintResources/StandardMacros.FlipFlop`)
    (:`A`
      _)
    (:`B`
      _))
  (set `self.Text Visibility` _isa))

(event `Info Panel`)

(fn `UserConstructionScript`)